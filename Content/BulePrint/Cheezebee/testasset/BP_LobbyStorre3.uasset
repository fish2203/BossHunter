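; BP_LobbyStorre3 is a lobby store actor that shows the player's store UI when the player comes close.
; On BeginPlay it caches player 0 as a BossHunterCharacter.
; Each Tick it measures the distance to that player, showing the WidgetSwitcher in the character's AllPlayerStoreWidget within a short fixed radius and hiding it otherwise, with no overlap events used.
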(event EventBeginPlay
  (bind _asboss_hunter_character (Utilities|Casting|CastToBossHunterCharacter (Game|GetPlayerCharacter 0)))
  (Variables|Default|Setplayer _asboss_hunter_character))

(event Collision|EventActorBeginOverlap
  (params (OtherActor :type Actor%20Object%20Reference)))

(event EventTick
  (params (DeltaSeconds :type Float%20%28single-precision%29))
  (bind _player (Variables|Default|Getplayer))
  (bind _allplayerstorewidget (Variables|/Script/BossHunter.BossHunterCharacter|GetallPlayerStoreWidget _player))
  (bind _widgetswitcher (Variables|/Script/BossHunter.StoreWidget|GetWidgetSwitcher _allplayerstorewidget))
  (if (< (Math|Vector|Distance(Vector) (Transformation|GetActorLocation) (Transformation|GetActorLocation (Variables|Default|Getplayer))) 2e+02)
    (Variables|/Script/UMG.Widget|SetVisibility _widgetswitcher "Visible")
    (else
      (Variables|/Script/UMG.Widget|SetVisibility _widgetswitcher "Hidden"))))

(fn ConstructionScript)